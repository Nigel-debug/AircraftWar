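; BP_Bullet is a bullet actor in AircraftWar that damages the first actor overlapping its sphere.
; A life span set on BeginPlay removes it if nothing is hit.
; The sphere overlap passes through a DoOnce, applies damage credited to the instigator's controller, then disables collision and hides the bullet before a short delay and destroy.
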(event `self.ReceiveBeginPlay`
  (`self.SetLifeSpan` 5.0))

(event `self.Sphere.OnComponentBeginOverlap`
  (params (OverlappedComponent :type "PrimitiveComponent Object Reference") (OtherActor :type "Actor Object Reference") (OtherComp :type "PrimitiveComponent Object Reference") (OtherBodyIndex :type Integer) (bFromSweep :type Boolean) (SweepResult :type "HitResult Structure (by ref)"))
  (`/Engine/EditorBlueprintResources/StandardMacros.DoOnce` false
    (:`Completed`
      (`GameplayStatics.ApplyDamage` OtherActor (`self.damageAmount`) (`self.GetInstigatorController`) self)
      (`PrimitiveComponent.SetCollisionEnabled` (`self.Sphere`) "NoCollision")
      (`SceneComponent.SetVisibility` (`self.DefaultSceneRoot`) false true)
      (`KismetSystemLibrary.Delay` 0.2)
      (`self.K2_DestroyActor`))))

(fn `UserConstructionScript`)