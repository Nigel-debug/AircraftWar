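; Homing rocket actor that chases a Target, applies damage on its first overlap and sets off the player pilot's alarm when that player is the target.
; Each tick it accelerates forward and turns toward the target, dropping the lock once the pitch offset passes a limit.
; Impact or a lifetime timer triggers Explosion, which hides the rocket, spawns effects, sound and camera shake, clears the alarm and schedules delayed destruction.
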(event `self.ReceiveBeginPlay`
  (`KismetSystemLibrary.K2_SetTimer` null "Explosion" 30.0)
  (bind _asbp_pilot (cast `/Game/AircraftWar/blueprint/BP_Pilot` (`GameplayStatics.GetPlayerPawn` 0)))
  (`/Engine/EditorBlueprintResources/StandardMacros.IsValid` _asbp_pilot
    (:`Is Valid`
      (set `self.OurPawn` _asbp_pilot)
      (`KismetSystemLibrary.Delay` 0.1)
      (`self.SetAlarmState` true))))

(event `self.ReceiveTick`
  (params (DeltaSeconds :type "Float (single-precision)"))
  (if (not (`self.isExploded`))
    (`self.SetSpeed` DeltaSeconds)
    (`self.PathFinder`)))

(event `self.Sphere.OnComponentBeginOverlap`
  (params (OverlappedComponent :type "PrimitiveComponent Object Reference") (OtherActor :type "Actor Object Reference") (OtherComp :type "PrimitiveComponent Object Reference") (OtherBodyIndex :type Integer) (bFromSweep :type Boolean) (SweepResult :type "HitResult Structure (by ref)"))
  (`/Engine/EditorBlueprintResources/StandardMacros.DoOnce` false
    (:`Completed`
      (`self.Explosion`)
      (`GameplayStatics.ApplyDamage` OtherActor (`self.damageAmount`) (`self.GetInstigatorController`) self)
      (`PrimitiveComponent.SetCollisionEnabled` (`self.Sphere`) "NoCollision"))))

(fn `destroyRocket`
  (`self.K2_DestroyActor`))

(fn `Explosion`
  (bind _returnvalue (`self.K2_GetActorLocation`))
  (if (not (`self.isExploded`))
    (`self.SetAlarmState` false)
    (set `self.isExploded` true)
    (`PrimitiveComponent.SetCollisionEnabled` (`self.Sphere`) "NoCollision")
    (`ActorComponent.Deactivate` (`self.engine`))
    (`SceneComponent.SetVisibility` (`self.DefaultSceneRoot`) false true)
    (`ActorComponent.Deactivate` (`self.smoke`))
    (`GameplayStatics.SpawnEmitterAtLocation` "/Game/AircraftWar/Effects/P_Explosion.P_Explosion" _returnvalue)
    (`GameplayStatics.SpawnSoundAtLocation` "/Game/AircraftWar/Cues/S_Explosion_Cue.S_Explosion_Cue" _returnvalue (struct) 2.0 1.0 0.0 "/Game/AircraftWar/Cues/A_Attenuation.A_Attenuation" null)
    (`GameplayStatics.PlayWorldCameraShake` "/Game/AircraftWar/blueprint/BP_ExplosionShake.BP_ExplosionShake_C" (`self.K2_GetActorLocation`) 10000.0)
    (`KismetSystemLibrary.K2_SetTimer` null "destroyRocket" 10.0)))

(fn `PathFinder`
  (locals (rotationTarget :type "Rotator Structure" :default (struct)) (TargetLocation :type "Vector Structure"))
  (bind _returnvalue (`self.K2_GetActorRotation`))
  (bind _target (`self.Target`))
  (bind _returnvalue_2 (`KismetMathLibrary.FindLookAtRotation` (`self.K2_GetActorLocation`) (`local.TargetLocation`)))
  (bind (_returnvalue_roll _returnvalue_pitch) (`KismetMathLibrary.BreakRotator` (`KismetMathLibrary.NormalizedDeltaRotator` _returnvalue _returnvalue_2)))
  (`/Engine/EditorBlueprintResources/StandardMacros.IsValid` _target
    (:`Is Valid`
      (set `local.TargetLocation` (`self.K2_GetActorLocation` _target))
      (if (and (<= _returnvalue_pitch 60.0) (<= _returnvalue_pitch 60.0))
        (set `local.rotationTarget` (`KismetMathLibrary.RInterpTo_Constant` _returnvalue _returnvalue_2 (`GameplayStatics.GetWorldDeltaSeconds`) (`self.interpRotation`)))
        (else
          (`self.SetAlarmState` false)
          (set `self.Target` null)))
      (`self.K2_SetActorRotation` (`local.rotationTarget`)))))

(fn `SetAlarmState`
  (params (turnOn :type Boolean))
  (if (== (`self.OurPawn`) (`self.Target`))
    (bind _asbp_pilot (cast `/Game/AircraftWar/blueprint/BP_Pilot` (`GameplayStatics.GetPlayerPawn` 0)))
    (`/Engine/EditorBlueprintResources/StandardMacros.IsValid` _asbp_pilot
      (:`Is Valid`
        (`/Game/AircraftWar/blueprint/BP_Pilot.SetAlarm` _asbp_pilot turnOn)))))

(fn `SetSpeed`
  (params (deltaTime :type "Float (double-precision)"))
  (bind _currentspeed (`self.currentSpeed`))
  (bind _maxspeed (`self.maxSpeed`))
  (if (< _currentspeed _maxspeed)
    (set `self.currentSpeed` (`KismetMathLibrary.FInterpTo_Constant` _currentspeed _maxspeed deltaTime (* (+ (`KismetMathLibrary.Abs` (/ _currentspeed _maxspeed)) 1.0) (`self.SpeedInterp`))))
    (else
      (set `self.currentSpeed` (`self.maxSpeed`))))
  (`self.K2_AddActorLocalOffset` (`KismetMathLibrary.MakeVector` (* deltaTime (`self.currentSpeed`))) true))

(fn `UserConstructionScript`)