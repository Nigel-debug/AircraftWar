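; BP_GM is the aircraft war game manager that sets up a two-team air battle at BeginPlay.
; It sorts PlayerStarts into A and B points by tag, then spawns numbered BP_AI planes for both teams with random X and Z offsets.
; After a short delay it replaces the player's pawn with a possessed BP_Pilot on team A and prints flight control hints.
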(event `self.ReceiveBeginPlay`
  (`self.GetSpawnPoints`)
  (`KismetSystemLibrary.Delay` 1.0)
  (`self.MultiSpawnAI`)
  (`KismetSystemLibrary.Delay` 0.5)
  (`self.SpawnPlayer` "A")
  (`KismetSystemLibrary.PrintString` "Right shift + Spacebar to control speed" true true (struct :`R` 1.0 :`G` 0.8919 :`A` 1.0) 30.0)
  (`KismetSystemLibrary.PrintString` "Q + E keys to control yaw" true true (struct :`R` 1.0 :`G` 0.414395 :`A` 1.0) 30.0))

(fn `GetSpawnPoints`
  (bind _outactors (`GameplayStatics.GetAllActorsOfClass` "/Script/Engine.PlayerStart"))
  (for _array_element _outactors
    (switch `name` (`PlayerStart.PlayerStartTag` _array_element)
      (:`A`
        (`KismetArrayLibrary.Array_AddUnique` (`self.Point_A`) _array_element))
      (:`B`
        (`KismetArrayLibrary.Array_AddUnique` (`self.Point_B`) _array_element)))))

(fn `MultiSpawnAI`
  (locals (ID :type Integer :default 2))
  (bind _ai_teamanumber (`self.AI_teamANumber`))
  (bind _returnvalue (+ _ai_teamanumber 1))
  (for _index (range (`local.ID`) (+ _returnvalue 1))
    (bind _output_get (set `local.ID` _index))
    (`self.SpawnAI` "A" _output_get))
  (bind _output_get_2 (set `local.ID` (+ _returnvalue 1)))
  (for _index_2 (range _output_get_2 (+ (+ _ai_teamanumber (`self.AI_teamBNumber`) 1) 1))
    (bind _output_get_3 (set `local.ID` _index_2))
    (`self.SpawnAI` "B" _output_get_3)))

(fn `SpawnAI`
  (params (setTeam :type Name) (setId :type Integer))
  (locals (ID :type Integer :default 2) (team :type Name))
  (bind _id (`local.ID`))
  (set `local.team` setTeam)
  (set `local.ID` setId)
  (bind (_location _rotation) (`self.spawnLocationRandomize` (`local.team`)))
  (bind _returnvalue (`|SpawnActorFromClass` "/Game/AircraftWar/blueprint/BP_AI.BP_AI_C" (`KismetMathLibrary.MakeTransform` _location _rotation) "AdjustIfPossibleButAlwaysSpawn" "OverrideRootScale" null null))
  (`/Engine/EditorBlueprintResources/StandardMacros.IsValid` _returnvalue
    (:`Is Valid`
      (`BlueprintMapLibrary.Map_Add` (`self.AI_Pawn`) _id)
      (`/Game/AircraftWar/blueprint/BP_AI.DefinePlayerInfo` _returnvalue (`local.team`) _id))))

(fn `spawnLocationRandomize`
  (params (Team :type Name) (ID :type Integer))
  (returns (Location :type "Vector Structure") (Rotation :type "Rotator Structure"))
  (locals (randomFactor :type Integer) (ID_AI :type Integer))
  (bind _returnvalue (`KismetMathLibrary.Conv_IntToDouble` (`local.randomFactor`)))
  (bind _returnvalue_2 (`KismetMathLibrary.Conv_IntToDouble` (`local.randomFactor`)))
  (bind _output (`|GetArrayItem` (`self.Point_B`)))
  (bind _output_2 (`|GetArrayItem` (`self.Point_A`)))
  (bind (_returnvalue_x _returnvalue_y _returnvalue_z) (`KismetMathLibrary.BreakVector` (`self.K2_GetActorLocation` _output)))
  (bind (_returnvalue_x_2 _returnvalue_y_2 _returnvalue_z_2) (`KismetMathLibrary.BreakVector` (`self.K2_GetActorLocation` _output_2)))
  (set `local.ID_AI` ID)
  (set `local.randomFactor` (`KismetMathLibrary.RandomIntegerInRange` -10000 10000))
  (switch `name` Team
    (:`Default`
      (return (0.0 0.0 0.0)))
    (:`A`
      (return (`KismetMathLibrary.MakeVector` (+ _returnvalue_x_2 _returnvalue_2) (+ _returnvalue_y_2 (`KismetMathLibrary.Conv_IntToDouble` (* 1500 (`local.ID_AI`)))) (+ _returnvalue_z_2 _returnvalue_2)) (`self.K2_GetActorRotation` _output_2)))
    (:`B`
      (return (`KismetMathLibrary.MakeVector` (+ _returnvalue_x _returnvalue) (+ _returnvalue_y (`KismetMathLibrary.Conv_IntToDouble` (* 1500 (`local.ID_AI`)))) (+ _returnvalue_z _returnvalue)) (`self.K2_GetActorRotation` _output)))))

(fn `SpawnPlayer`
  (params (Team :type Name))
  (locals (spawn_transform :type "Transform Structure") (my_team :type Name))
  (bind _returnvalue (`GameplayStatics.GetPlayerController` 0))
  (bind _returnvalue_2 (`Controller.K2_GetPawn` _returnvalue))
  (bind _output (`|GetArrayItem` (`self.Point_B`)))
  (bind _output_2 (`|GetArrayItem` (`self.Point_A`)))
  (bind _output_get (set `local.my_team` Team))
  (switch `name` _output_get
    (:`A`
      (`/Engine/EditorBlueprintResources/StandardMacros.IsValid` _output_2
        (:`Is Valid`
          (set `local.spawn_transform` (`self.GetTransform` _output_2)))))
    (:`B`
      (`/Engine/EditorBlueprintResources/StandardMacros.IsValid` _output
        (:`Is Valid`
          (set `local.spawn_transform` (`self.GetTransform` _output))))))
  (`/Engine/EditorBlueprintResources/StandardMacros.IsValid` _returnvalue_2
    (:`Is Valid`
      (`self.K2_DestroyActor` _returnvalue_2))
    (:`Is Not Valid`
      _))
  (bind _returnvalue_3 (`|SpawnActorFromClass` "/Game/AircraftWar/blueprint/BP_Pilot.BP_Pilot_C" (`local.spawn_transform`) "AdjustIfPossibleButAlwaysSpawn" "OverrideRootScale" null null))
  (`Controller.Possess` _returnvalue _returnvalue_3)
  (`/Engine/EditorBlueprintResources/StandardMacros.IsValid` _returnvalue_3
    (:`Is Valid`
      (`/Game/AircraftWar/blueprint/BP_Pilot.DefinePlayerInfo` _returnvalue_3 (`local.my_team`) 1))))

(fn `UserConstructionScript`)