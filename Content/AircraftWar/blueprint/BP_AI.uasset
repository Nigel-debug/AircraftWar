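; AI-controlled fighter jet for a two-team air war that hunts enemies, fires guns and target-assigned rockets, and respawns after exploding.
; Each Tick it flies forward, sphere-traces for a target, then PathFinder steers toward it or the WarZone, firing when aligned and close.
; Overlap sensors override steering with timed climbs or side turns, while banking adjusts speed and turn rate.
; Pawn versus PhysicsBody object types separate teams, registered with BP_HUD.
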(event `InputAxis|speed`
  (params (AxisValue :type "Float (single-precision)"))
  (bind _currentspeed (`self.currentSpeed`))
  (bind _sound_engine (`self.Sound_Engine`))
  (bind _targetspeed (`self.targetSpeed`))
  (bind _returnvalue (- (`self.targetSpeed`) (`self.currentSpeed`)))
  (bind _returnvalue_2 (/ (`self.currentSpeed`) (`self.maxSpeed`)))
  ;[1 1 1] speed
  (if (>= (`KismetMathLibrary.Abs` AxisValue) 0.1)
    (set `self.targetSpeed` (`KismetMathLibrary.FInterpTo_Constant` (`self.targetSpeed`) (* AxisValue (`self.maxSpeed`)) (`GameplayStatics.GetWorldDeltaSeconds`) (`self.SpeedInterp`))))
  (if (< (`self.targetSpeed`) (`self.MinSpeed`))
    (set `self.targetSpeed` (`self.MinSpeed`)))
  (if (!= (`self.targetSpeed`) (`self.currentSpeed`))
    (set `self.currentSpeed` (`KismetMathLibrary.FInterpTo_Constant` _currentspeed _targetspeed (`GameplayStatics.GetWorldDeltaSeconds`) (* (+ (`KismetMathLibrary.Abs` (/ (- _currentspeed _targetspeed) (`self.maxSpeed`))) 0.2) (`self.SpeedInterp`)))))
  (`AudioComponent.SetPitchMultiplier` _sound_engine _returnvalue_2)
  (`AudioComponent.SetVolumeMultiplier` _sound_engine (* _returnvalue_2 0.5))
  (set `self.acceleration` (/ _returnvalue (`KismetMathLibrary.Abs` _returnvalue))))

(event `self.ReceiveBeginPlay`
  (bind (_returnvalue_x _returnvalue_y _returnvalue_z) (`KismetMathLibrary.BreakVector` (`self.K2_GetActorLocation`)))
  (bind _flyexperience (`self.FlyExperience`))
  ;[1 1 1] begin
  (bind _output_get (set `self.targetSpeed` (`self.MinSpeed`)))
  (set `self.currentSpeed` _output_get)
  (set `self.MySpawnPoint` (`self.GetTransform`))
  (set `self.FlyExperience` (`KismetMathLibrary.RandomFloatInRange` _flyexperience (+ _flyexperience 1.0)))
  (bind _outactors (`GameplayStatics.GetAllActorsOfClass` "/Script/Engine.PlayerStart"))
  (for _array_element _outactors
    (if (== (`PlayerStart.PlayerStartTag` _array_element) "WarZone")
      (bind (_returnvalue_x_2 _returnvalue_y_2 _returnvalue_z_2) (`KismetMathLibrary.BreakVector` (`self.K2_GetActorLocation` _array_element)))
      (set `self.WarZoneLocation` (`KismetMathLibrary.MakeVector` (+ (- _returnvalue_x _returnvalue_x_2) _returnvalue_x_2) _returnvalue_y_2 (+ (- _returnvalue_z _returnvalue_z_2) _returnvalue_z_2))))))

(event `self.ReceiveTick`
  (params (DeltaSeconds :type "Float (single-precision)"))
  ;[1 1 1] event tick
  (if (not (`self.isDead`))
    (`self.ForwardMovement` DeltaSeconds)
    (`self.GetTarget`)
    (`self.PathFinder`)))

(event `self.ReceiveAnyDamage`
  (params (Damage :type "Float (single-precision)") (DamageType :type "DamageType Object Reference") (InstigatedBy :type "Controller Object Reference") (DamageCauser :type "Actor Object Reference"))
  (bind _returnvalue (- (`self.health`) Damage))
  ;[1 1 1] weapons and damage
  (`/Engine/EditorBlueprintResources/StandardMacros.IsValid` DamageCauser
    (:`Is Valid`
      (if (<= _returnvalue 0.0)
        (`self.Explode`)
        (else
          (set `self.health` _returnvalue))))))

(event `InputAction|shoot_rocket`
  (params (Key :type "Key Structure"))
  ;[1 1 1] weapons and damage
  (:`Pressed`
    (`self.FireRocket`)))

(event `self.Jet.OnComponentBeginOverlap`
  (params (OverlappedComponent :type "PrimitiveComponent Object Reference") (OtherActor :type "Actor Object Reference") (OtherComp :type "PrimitiveComponent Object Reference") (OtherBodyIndex :type Integer) (bFromSweep :type Boolean) (SweepResult :type "HitResult Structure (by ref)"))
  ;[1 1 1] overlap
  (`/Engine/EditorBlueprintResources/StandardMacros.IsValid` OtherActor
    (:`Is Valid`
      (if (== (`|GetArrayItem` (`Actor.Tags` OtherActor)) "None")
        (`self.Explode`)
        (`KismetSystemLibrary.PrintString` (`KismetSystemLibrary.GetDisplayName` OtherActor) true true (struct :`R` 1.0 :`B` 0.042602 :`A` 1.0) 30.0)))))

(event `InputAction|shoot_bullet`
  (params (Key :type "Key Structure"))
  (bind _audiomachinegun (`self.AudioMachineGun`))
  (bind _muzzle (`self.muzzle`))
  ;[1 1 1] weapons and damage
  (:`Pressed`
    (set `self.isFiringBullet` true)
    (`self.FireBullet`)
    (`ActorComponent.Activate` _muzzle true)
    (`AudioComponent.Play` _audiomachinegun 0.0))
  (:`Released`
    (set `self.isFiringBullet` false)
    (`ActorComponent.Deactivate` _muzzle)
    (`AudioComponent.Stop` _audiomachinegun)))

(event `self.ObstacleDetect.OnComponentBeginOverlap`
  (params (OverlappedComponent :type "PrimitiveComponent Object Reference") (OtherActor :type "Actor Object Reference") (OtherComp :type "PrimitiveComponent Object Reference") (OtherBodyIndex :type Integer) (bFromSweep :type Boolean) (SweepResult :type "HitResult Structure (by ref)"))
  (set `self.FrontObstacle` true)
  (`KismetSystemLibrary.K2_SetTimer` null "endFrontObstacle" 2.0))

(event `self.RightObstacleDetect.OnComponentBeginOverlap`
  (params (OverlappedComponent :type "PrimitiveComponent Object Reference") (OtherActor :type "Actor Object Reference") (OtherComp :type "PrimitiveComponent Object Reference") (OtherBodyIndex :type Integer) (bFromSweep :type Boolean) (SweepResult :type "HitResult Structure (by ref)"))
  (bind _sideobstacle (`self.SideObstacle`))
  (if (or (== _sideobstacle 0) (== _sideobstacle 1))
    (set `self.SideObstacle` 1)
    (`KismetSystemLibrary.K2_SetTimer` null "endSideObstacle" 3.0)))

(event `self.LeftObstacleDetect.OnComponentBeginOverlap`
  (params (OverlappedComponent :type "PrimitiveComponent Object Reference") (OtherActor :type "Actor Object Reference") (OtherComp :type "PrimitiveComponent Object Reference") (OtherBodyIndex :type Integer) (bFromSweep :type Boolean) (SweepResult :type "HitResult Structure (by ref)"))
  (bind _sideobstacle (`self.SideObstacle`))
  (if (or (== _sideobstacle 0) (== _sideobstacle 2))
    (set `self.SideObstacle` 2)
    (`KismetSystemLibrary.K2_SetTimer` null "endSideObstacle" 3.0)))

(fn `DefinePlayerInfo`
  (params (Team :type Name) (Player_ID :type Integer))
  (bind _jet (`self.Jet`))
  (bind (_asbp_hud _bsuccess) (cast `/Game/AircraftWar/blueprint/BP_HUD` (`PlayerController.GetHUD` (`GameplayStatics.GetPlayerController` 0)) :!pure true))
  (bind (_asbp_hud_2 _bsuccess_2) (cast `/Game/AircraftWar/blueprint/BP_HUD` (`PlayerController.GetHUD` (`GameplayStatics.GetPlayerController` 0)) :!pure true))
  (bind _output_get (set `self.Player_ID` Player_ID))
  (`KismetArrayLibrary.Array_Insert` (`self.Tags`) (`KismetStringLibrary.Conv_StringToName` (`KismetStringLibrary.Conv_IntToString` _output_get)))
  (bind _output_get_2 (set `self.Team` Team))
  (set `self.isDead` false)
  (set `self.health` (`self.maxHealth`))
  (`SceneComponent.SetVisibility` (`self.DefaultSceneRoot`) true true)
  (switch `name` _output_get_2
    (:`A`
      (`PrimitiveComponent.SetCollisionObjectType` _jet "ECC_Pawn")
      (`PrimitiveComponent.SetCollisionEnabled` _jet "QueryAndPhysics")
      (if _bsuccess
        (`KismetArrayLibrary.Array_AddUnique` (`/Game/AircraftWar/blueprint/BP_HUD.ActorsTeamA` _asbp_hud) self)))
    (:`B`
      (`PrimitiveComponent.SetCollisionObjectType` _jet "ECC_PhysicsBody")
      (`PrimitiveComponent.SetCollisionEnabled` _jet "QueryAndPhysics")
      (if _bsuccess_2
        (`KismetArrayLibrary.Array_AddUnique` (`/Game/AircraftWar/blueprint/BP_HUD.ActorsTeamB` _asbp_hud_2) self)))))

(fn `endFrontObstacle`
  (set `self.FrontObstacle` false)
  (`KismetSystemLibrary.PrintString` "clear obstacle" true true (struct :`G` 0.66 :`B` 1.0 :`A` 1.0) 20.0))

(fn `endSideObstacle`
  (set `self.SideObstacle` 0)
  (`KismetSystemLibrary.PrintString` "clear obstacle" true true (struct :`G` 0.66 :`B` 1.0 :`A` 1.0) 20.0))

(fn `Explode`
  (bind _returnvalue (`self.K2_GetActorLocation`))
  (bind (_asbp_hud _bsuccess) (cast `/Game/AircraftWar/blueprint/BP_HUD` (`PlayerController.GetHUD` (`GameplayStatics.GetPlayerController` 0)) :!pure true))
  (if (not (`self.isDead`))
    (`KismetArrayLibrary.Array_Insert` (`self.Tags`) "0")
    (set `self.isFiringBullet` false)
    (set `self.isDead` true)
    (`PrimitiveComponent.SetCollisionEnabled` (`self.Jet`) "NoCollision")
    (`GameplayStatics.SpawnEmitterAtLocation` "/Game/AircraftWar/Effects/P_Explosion.P_Explosion" _returnvalue)
    (`GameplayStatics.SpawnSoundAtLocation` "/Game/AircraftWar/Cues/S_Explosion_Cue.S_Explosion_Cue" _returnvalue (struct) 2.0 1.0 0.0 "/Game/AircraftWar/Cues/A_Attenuation.A_Attenuation" null)
    (`SceneComponent.SetVisibility` (`self.DefaultSceneRoot`) false true)
    (`KismetSystemLibrary.K2_SetTimer` null "RespawnAI" (`self.respawnTime`))
    (if _bsuccess
      (`KismetArrayLibrary.Array_RemoveItem` (`/Game/AircraftWar/blueprint/BP_HUD.ActorsTeamA` _asbp_hud) self)
      (`KismetArrayLibrary.Array_RemoveItem` (`/Game/AircraftWar/blueprint/BP_HUD.ActorsTeamB` _asbp_hud) self)
      (`GameplayStatics.PlayWorldCameraShake` "/Game/AircraftWar/blueprint/BP_ExplosionShake.BP_ExplosionShake_C" (`self.K2_GetActorLocation`) 10000.0))))

(fn `FireBullet`
  (bind _returnvalue (`SceneComponent.K2_GetComponentToWorld` (`self.muzzle`)))
  (if (`self.isDead`)
    _
    (elif (`self.isFiringBullet`)
      (bind _returnvalue_2 (`|SpawnActorFromClass` "/Game/AircraftWar/blueprint/BP_Bullet.BP_Bullet_C" (`KismetMathLibrary.MakeTransform` (.location _returnvalue) (`KismetMathLibrary.MakeRotator` (.roll (.rotation _returnvalue)) (+ (.pitch (.rotation _returnvalue)) (`KismetMathLibrary.RandomFloatInRange` -0.5 1.0)) (+ (.yaw (.rotation _returnvalue)) (`KismetMathLibrary.RandomFloatInRange` -0.5 1.0)))) "Undefined" "OverrideRootScale" null null))
      (`/Engine/EditorBlueprintResources/StandardMacros.IsValid` _returnvalue_2
        (:`Is Valid`
          (`KismetArrayLibrary.Array_Insert` (`Actor.Tags` _returnvalue_2) (`KismetStringLibrary.Conv_StringToName` (`KismetStringLibrary.Conv_IntToString` (`self.Player_ID`))))
          (if (`|EnumEquality` (`PrimitiveComponent.GetCollisionObjectType` (`self.Jet`)) "ECC_Pawn")
            (bind _sphere (`/Game/AircraftWar/blueprint/BP_Bullet.Sphere` _returnvalue_2))
            (`PrimitiveComponent.SetCollisionResponseToChannel` _sphere "ECC_PhysicsBody" "ECR_Overlap")
            (else
              (`PrimitiveComponent.SetCollisionResponseToChannel` _sphere "ECC_Pawn" "ECR_Overlap"))))
        (:`Is Not Valid`
          _))
      (`KismetSystemLibrary.K2_SetTimer` null "FireBullet" (`self.shootingSpeed`)))))

(fn `FireRocket`
  (bind _r_rocket (`self.R_rocket`))
  (bind _l_rocket (`self.L_rocket`))
  (if (== (`self.RocketSpawnedID`) 0)
    (if (and (`SceneComponent.IsVisible` _r_rocket) (`SceneComponent.IsVisible` (`self.L_rocket`)))
      (set `self.RocketSpawnedID` 1)
      (set `self.spawnrocketTransform` (`SceneComponent.K2_GetComponentToWorld` _r_rocket))
      (`SceneComponent.SetVisibility` _r_rocket false false)
      (`|ExecutionSequence`
        (:`then_0`
          (bind _returnvalue (`|SpawnActorFromClass` "/Game/AircraftWar/blueprint/BP_rocket.BP_rocket_C" (`self.spawnrocketTransform`) "Undefined" "OverrideRootScale" null null :!label _label))
          (`/Engine/EditorBlueprintResources/StandardMacros.IsValid` _returnvalue
            (:`Is Valid`
              (`KismetArrayLibrary.Array_Insert` (`Actor.Tags` _returnvalue) (`KismetStringLibrary.Conv_StringToName` (`KismetStringLibrary.Conv_IntToString` (`self.Player_ID`))))
              (set `/Game/AircraftWar/blueprint/BP_rocket.currentSpeed` (`self.currentSpeed`) _returnvalue)
              (if (`|EnumEquality` (`PrimitiveComponent.GetCollisionObjectType` (`self.Jet`)) "ECC_Pawn")
                (bind _sphere (`/Game/AircraftWar/blueprint/BP_rocket.Sphere` _returnvalue))
                (`PrimitiveComponent.SetCollisionResponseToChannel` _sphere "ECC_PhysicsBody" "ECR_Overlap")
                (else
                  (`PrimitiveComponent.SetCollisionResponseToChannel` _sphere "ECC_Pawn" "ECR_Overlap")))
              (`GameplayStatics.SpawnSoundAtLocation` "/Game/AircraftWar/Cues/S_Missile_engine_Cue.S_Missile_engine_Cue" (`self.K2_GetActorLocation`) (struct) 3.0 1.0 0.0 "/Game/AircraftWar/Cues/A_Attenuation.A_Attenuation" null)
              (set `/Game/AircraftWar/blueprint/BP_rocket.Target` (`self.MyTarget`) _returnvalue))))
        (:`then_1`
          (`KismetSystemLibrary.K2_SetTimer` null "ReloadRocket" (`self.reloadRocketTime`)))))
    (elif (and (`SceneComponent.IsVisible` _l_rocket) (`SceneComponent.IsVisible` (`self.R_rocket`)))
      (set `self.RocketSpawnedID` 0)
      (set `self.spawnrocketTransform` (`SceneComponent.K2_GetComponentToWorld` _l_rocket))
      (`SceneComponent.SetVisibility` _l_rocket false false)
      (`|ExecutionSequence`
        (:`then_0`
          (goto _label))
        (:`then_1`
          (`KismetSystemLibrary.K2_SetTimer` null "ReloadRocket" (`self.reloadRocketTime`)))))))

(fn `ForwardMovement`
  (params (deltaTime :type "Float (double-precision)"))
  (`self.K2_AddActorLocalOffset` (`KismetMathLibrary.MakeVector` (* deltaTime (`self.currentSpeed`))) true))

(fn `GetTarget`
  (bind _returnvalue (`self.K2_GetActorLocation`))
  (`/Engine/EditorBlueprintResources/StandardMacros.IsValid` (`self.MyTarget`)
    (:`Is Not Valid`
      (if (`|EnumEquality` (`PrimitiveComponent.GetCollisionObjectType` (`self.Jet`)) "ECC_Pawn")
        (bind _outhit (`KismetSystemLibrary.SphereTraceSingleForObjects` _returnvalue _returnvalue 5000.0 (`|MakeArray` "ObjectTypeQuery4" :!type "EObjectTypeQuery Enum")))
        (set `self.MyTarget` (`.HitActor` (`GameplayStatics.BreakHitResult` _outhit)))
        (else
          (bind _outhit_2 (`KismetSystemLibrary.SphereTraceSingleForObjects` _returnvalue _returnvalue 5000.0 (`|MakeArray` "ObjectTypeQuery3" :!type "EObjectTypeQuery Enum")))
          (set `self.MyTarget` (`.HitActor` (`GameplayStatics.BreakHitResult` _outhit_2))))))))

(fn `PathFinder`
  (locals (TargetLocation :type "Vector Structure") (TargetRotation :type "Rotator Structure") (targetPitch :type "Float (double-precision)" :default 0.0))
  (bind (_returnvalue_roll _returnvalue_pitch _returnvalue_yaw) (`KismetMathLibrary.BreakRotator` (`self.K2_GetActorRotation`)))
  (bind _returnvalue (`self.K2_GetActorLocation`))
  (bind (_returnvalue_roll_2 _returnvalue_pitch_2 _returnvalue_yaw_2) (`KismetMathLibrary.BreakRotator` (`self.K2_GetActorRotation`)))
  (bind (_returnvalue_roll_3 _returnvalue_pitch_3 _returnvalue_yaw_3) (`KismetMathLibrary.BreakRotator` (`self.K2_GetActorRotation`)))
  (bind (_returnvalue_roll_4 _returnvalue_pitch_4 _returnvalue_yaw_4) (`KismetMathLibrary.BreakRotator` (`self.K2_GetActorRotation`)))
  (bind _mytarget (`self.MyTarget`))
  (bind _targetlocation (`local.TargetLocation`))
  (bind (_returnvalue_roll_5 _returnvalue_pitch_5 _returnvalue_yaw_5) (`KismetMathLibrary.BreakRotator` (`KismetMathLibrary.FindLookAtRotation` _returnvalue _targetlocation)))
  (bind _returnvalue_2 (- _returnvalue_yaw_3 60.0))
  (bind (_returnvalue_roll_6 _returnvalue_pitch_6 _returnvalue_yaw_6) (`KismetMathLibrary.BreakRotator` (`KismetMathLibrary.RInterpTo_Constant` (`KismetMathLibrary.MakeRotator` _returnvalue_roll_4 _returnvalue_pitch_4 _returnvalue_yaw_4) (`KismetMathLibrary.MakeRotator` 0.0 (`local.targetPitch`) _returnvalue_yaw_4) (`GameplayStatics.GetWorldDeltaSeconds`) (`self.interpRotation`))))
  (bind (_returnvalue_roll_7 _returnvalue_pitch_7 _returnvalue_yaw_7) (`KismetMathLibrary.BreakRotator` (`KismetMathLibrary.FindLookAtRotation` (`self.K2_GetActorLocation`) (`local.TargetLocation`))))
  (bind _returnvalue_3 (+ _returnvalue_yaw 60.0))
  (bind (_returnvalue_roll_8 _returnvalue_pitch_8 _returnvalue_yaw_8) (`KismetMathLibrary.BreakRotator` (`KismetMathLibrary.RInterpTo_Constant` (`self.K2_GetActorRotation`) (`KismetMathLibrary.MakeRotator` _returnvalue_roll_7 _returnvalue_pitch_7 _returnvalue_yaw_7) (`GameplayStatics.GetWorldDeltaSeconds`) (`self.interpRotation`))))
  (bind (_returnvalue_roll_9 _returnvalue_pitch_9 _returnvalue_yaw_9) (`KismetMathLibrary.BreakRotator` (`KismetMathLibrary.RInterpTo_Constant` (`KismetMathLibrary.MakeRotator` _returnvalue_roll_3 _returnvalue_pitch_3 _returnvalue_yaw_3) (`KismetMathLibrary.MakeRotator` 0.0 (`local.targetPitch`) _returnvalue_2) (`GameplayStatics.GetWorldDeltaSeconds`) (`self.interpRotation`))))
  (bind (_returnvalue_roll_10 _returnvalue_pitch_10 _returnvalue_yaw_10) (`KismetMathLibrary.BreakRotator` (`KismetMathLibrary.RInterpTo_Constant` (`KismetMathLibrary.MakeRotator` _returnvalue_roll _returnvalue_pitch _returnvalue_yaw) (`KismetMathLibrary.MakeRotator` 0.0 (`local.targetPitch`) _returnvalue_3) (`GameplayStatics.GetWorldDeltaSeconds`) (`self.interpRotation`))))
  (switch `int` (`self.SideObstacle`)
    (:`0`
      (if (`self.FrontObstacle`)
        (set `local.targetPitch` 80.0)
        (set `local.TargetRotation` (`KismetMathLibrary.MakeRotator` (`self.SpeedRollCalculation` _returnvalue_yaw_4) _returnvalue_pitch_6 _returnvalue_yaw_6))
        (else
          (`/Engine/EditorBlueprintResources/StandardMacros.IsValid` _mytarget
            (:`Is Valid`
              (if (== (`|GetArrayItem` (`Actor.Tags` _mytarget)) "0")
                (set `self.isFiringBullet` false :!label _label)
                (set `local.TargetLocation` (`self.WarZoneLocation`))
                (else
                  (set `local.TargetLocation` (`self.K2_GetActorLocation` _mytarget))
                  (if (and (<= (`KismetMathLibrary.Abs` (- _returnvalue_yaw_2 _returnvalue_yaw_5)) 20.0) (<= (`KismetMathLibrary.Abs` (- _returnvalue_pitch_5 _returnvalue_pitch_2)) 20.0) (<= (`KismetMathLibrary.VSize` (- _returnvalue _targetlocation)) 5000.0))
                    (set `self.isFiringBullet` true)
                    (`self.FireRocket`)
                    (else
                      (set `self.isFiringBullet` false)))
                  (`self.FireBullet`))))
            (:`Is Not Valid`
              (goto _label)))
          (set `local.TargetRotation` (`KismetMathLibrary.MakeRotator` (`self.SpeedRollCalculation` _returnvalue_yaw_7) _returnvalue_pitch_8 _returnvalue_yaw_8)))))
    (:`1`
      (set `self.isFiringBullet` false)
      (if (`self.FrontObstacle`)
        (set `local.targetPitch` 80.0)
        (else
          (set `local.targetPitch` 0.0)))
      (set `local.TargetRotation` (`KismetMathLibrary.MakeRotator` (`self.SpeedRollCalculation` _returnvalue_2) _returnvalue_pitch_9 _returnvalue_yaw_9)))
    (:`2`
      (set `self.isFiringBullet` false)
      (if (`self.FrontObstacle`)
        (set `local.targetPitch` 80.0)
        (else
          (set `local.targetPitch` 0.0)))
      (set `local.TargetRotation` (`KismetMathLibrary.MakeRotator` (`self.SpeedRollCalculation` _returnvalue_3) _returnvalue_pitch_10 _returnvalue_yaw_10))))
  (`self.K2_SetActorRotation` (`local.TargetRotation`)))

(fn `ReloadRocket`
  (`SceneComponent.SetVisibility` (`self.R_rocket`) true false)
  (`SceneComponent.SetVisibility` (`self.L_rocket`) true false))

(fn `RespawnAI`
  (`self.K2_SetActorTransform` (`self.MySpawnPoint`))
  (`self.DefinePlayerInfo` (`self.Team`) (`self.Player_ID`)))

(fn `RespawnPlayer`)

(fn `SpeedRollCalculation`
  (params (yaw :type "Float (double-precision)"))
  (returns (roll :type "Float (double-precision)"))
  (bind (_returnvalue_roll _returnvalue_pitch _returnvalue_yaw) (`KismetMathLibrary.BreakRotator` (`self.K2_GetActorRotation`)))
  (bind _returnvalue (`KismetMathLibrary.FClamp` (`KismetMathLibrary.Abs` (/ yaw (`self.FlyExperience`))) 10.0 20.0))
  (set `self.interpRotation` (`KismetMathLibrary.FInterpTo` (`self.interpRotation`) _returnvalue (`GameplayStatics.GetWorldDeltaSeconds`) 0.5))
  (set `self.currentSpeed` (`KismetMathLibrary.FClamp` (* (/ (`self.FlyExperience`) _returnvalue) (`self.maxSpeed`)) (`self.MinSpeed`) (`self.maxSpeed`)))
  (return (`KismetMathLibrary.FInterpTo` _returnvalue_roll (`KismetMathLibrary.FClamp` (- yaw _returnvalue_yaw) -60.0 60.0) (`GameplayStatics.GetWorldDeltaSeconds`) 1.0)))

(fn `UserConstructionScript`)