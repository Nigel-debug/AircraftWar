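; BP_Pilot is the player's jet pawn in AircraftWar, handling flight, weapons, damage and respawn.
; Interpolated axis inputs drive swept movement and rotation on Tick, plus spring-arm lag, engine audio and BP_HUD crosshair position.
; Timers repeat spread machine-gun fire, reload alternating rockets that follow the HUD's target, and respawn exploded jets at their start transform.
; Teams use Pawn or PhysicsBody object types so projectiles overlap only enemies.
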(event `InputAxis|speed`
  (params (AxisValue :type "Float (single-precision)"))
  (bind _currentspeed (`self.currentSpeed`))
  (bind _sound_engine (`self.Sound_Engine`))
  (bind _targetspeed (`self.targetSpeed`))
  (bind _returnvalue (- (`self.targetSpeed`) (`self.currentSpeed`)))
  (bind _returnvalue_2 (/ (`self.currentSpeed`) (`self.maxSpeed`)))
  ;[1 1 1] define speed , spring arm forward drag and  engine audio
  (if (>= (`KismetMathLibrary.Abs` AxisValue) 0.1)
    (set `self.targetSpeed` (`KismetMathLibrary.FInterpTo_Constant` (`self.targetSpeed`) (* AxisValue (`self.maxSpeed`)) (`GameplayStatics.GetWorldDeltaSeconds`) (`self.SpeedInterp`))))
  (if (< (`self.targetSpeed`) (`self.MinSpeed`))
    (set `self.targetSpeed` (`self.MinSpeed`)))
  (if (!= (`self.targetSpeed`) (`self.currentSpeed`))
    (set `self.currentSpeed` (`KismetMathLibrary.FInterpTo_Constant` _currentspeed _targetspeed (`GameplayStatics.GetWorldDeltaSeconds`) (* (+ (`KismetMathLibrary.Abs` (/ (- _currentspeed _targetspeed) (`self.maxSpeed`))) 0.2) (`self.SpeedInterp`)))))
  (set `SpringArmComponent.TargetArmLength` (* (+ (/ (`self.currentSpeed`) (* (`self.maxSpeed`) 5.0)) 1.0) (`self.springarmLengh`)) (`self.SpringArm`))
  (`AudioComponent.SetPitchMultiplier` _sound_engine _returnvalue_2)
  (`AudioComponent.SetVolumeMultiplier` _sound_engine (* _returnvalue_2 0.5))
  (set `self.acceleration` (/ _returnvalue (`KismetMathLibrary.Abs` _returnvalue))))

(event `self.ReceiveBeginPlay`
  ;[1 1 1] begin
  (bind _output_get (set `self.targetSpeed` (`self.MinSpeed`)))
  (set `self.currentSpeed` _output_get)
  ;;[1 1 1] we are using this point to respawn our pawn
  (set `self.MySpawnPoint` (`self.GetTransform`))
  (bind _returnvalue (`|CreateWidget` "/Game/AircraftWar/blueprint/UMG_PilotMenu.UMG_PilotMenu_C"))
  (set `self.PilotMenu` _returnvalue))

(event `self.ReceiveTick`
  (params (DeltaSeconds :type "Float (single-precision)"))
  ;[1 1 1] event tick
  (if (not (`self.isDead`))
    (`self.ForwardMovement` DeltaSeconds)
    (`self.RotationControl` DeltaSeconds)))

(event `InputAction|open_wheels`
  (params (Key :type "Key Structure"))
  ;[1 1 1] jet controll
  (:`Pressed`
    (if (`self.wheel_open`)
      (set `self.wheel_open` false)
      (else
        (set `self.wheel_open` true)))))

(event `InputAxis|yaw`
  (params (AxisValue :type "Float (single-precision)"))
  (bind _yaw_adder (`self.yaw_adder`))
  (bind _yaw_adder_2 (`self.yaw_adder`))
  ;[1 1 1] jet controll
  (set `self.yaw` AxisValue)
  (if (> (`KismetMathLibrary.Abs` (`self.yaw_adder`)) (`self.yaw_max`))
    (set `self.yaw_adder` (* (`self.yaw_max`) (/ _yaw_adder (`KismetMathLibrary.Abs` _yaw_adder))))
    (else
      (set `self.yaw_adder` (`KismetMathLibrary.FInterpTo_Constant` _yaw_adder_2 (* (`self.yaw`) (`self.yaw_max`)) (`GameplayStatics.GetWorldDeltaSeconds`) (+ (`KismetMathLibrary.Abs` _yaw_adder_2) (`self.interpYaw`)))))))

(event `self.ReceiveAnyDamage`
  (params (Damage :type "Float (single-precision)") (DamageType :type "DamageType Object Reference") (InstigatedBy :type "Controller Object Reference") (DamageCauser :type "Actor Object Reference"))
  (bind _pilotmenu (`self.PilotMenu`))
  (bind _returnvalue (- (`self.health`) Damage))
  ;[1 1 1] weapons and damage
  (`/Engine/EditorBlueprintResources/StandardMacros.IsValid` DamageCauser
    (:`Is Valid`
      (if (<= _returnvalue 0.0)
        (`self.Explode`)
        (else
          (set `self.health` _returnvalue)
          (`/Engine/EditorBlueprintResources/StandardMacros.IsValid` _pilotmenu
            (:`Is Valid`
              (`/Game/AircraftWar/blueprint/UMG_PilotMenu.SetHealth` _pilotmenu (/ (`self.health`) (`self.maxHealth`))))))))))

(event `InputAction|shoot_rocket`
  (params (Key :type "Key Structure"))
  ;[1 1 1] weapons and damage
  (:`Pressed`
    (if (not (`self.isDead`))
      (`self.FireRocket`))))

(event `InputAxis|pitch`
  (params (AxisValue :type "Float (single-precision)"))
  (bind _pitch_adder (`self.pitch_adder`))
  (bind _pitch_adder_2 (`self.pitch_adder`))
  ;[1 1 1] jet controll
  (set `self.pitch` AxisValue)
  (if (> (`KismetMathLibrary.Abs` (`self.pitch_adder`)) (`self.pitch_max`))
    (set `self.pitch_adder` (* (`self.pitch_max`) (/ _pitch_adder (`KismetMathLibrary.Abs` _pitch_adder))))
    (else
      (set `self.pitch_adder` (`KismetMathLibrary.FInterpTo_Constant` _pitch_adder_2 (* (`self.pitch`) (`self.pitch_max`)) (`GameplayStatics.GetWorldDeltaSeconds`) (+ (`KismetMathLibrary.Abs` _pitch_adder_2) (`self.interpPitch`)))))))

(event `self.Jet.OnComponentBeginOverlap`
  (params (OverlappedComponent :type "PrimitiveComponent Object Reference") (OtherActor :type "Actor Object Reference") (OtherComp :type "PrimitiveComponent Object Reference") (OtherBodyIndex :type Integer) (bFromSweep :type Boolean) (SweepResult :type "HitResult Structure (by ref)"))
  ;[1 1 1] overlap
  (`/Engine/EditorBlueprintResources/StandardMacros.IsValid` OtherActor
    (:`Is Valid`
      (if (== (`|GetArrayItem` (`Actor.Tags` OtherActor)) "None")
        (`self.Explode`)))))

(event `InputAxis|roll`
  (params (AxisValue :type "Float (single-precision)"))
  (bind _roll_adder (`self.roll_adder`))
  (bind _roll_adder_2 (`self.roll_adder`))
  ;[1 1 1] jet controll
  (set `self.roll` AxisValue)
  (if (> (`KismetMathLibrary.Abs` (`self.roll_adder`)) (`self.roll_max`))
    (set `self.roll_adder` (* (`self.roll_max`) (/ _roll_adder (`KismetMathLibrary.Abs` _roll_adder))))
    (else
      (set `self.roll_adder` (`KismetMathLibrary.FInterpTo_Constant` _roll_adder_2 (* (`self.roll`) (`self.roll_max`)) (`GameplayStatics.GetWorldDeltaSeconds`) (+ (`KismetMathLibrary.Abs` _roll_adder_2) (`self.interpRoll`)))))))

(event `InputAction|shoot_bullet`
  (params (Key :type "Key Structure"))
  (bind _audiomachinegun (`self.AudioMachineGun`))
  (bind _muzzle (`self.muzzle`))
  ;[1 1 1] weapons and damage
  (:`Pressed`
    (if (not (`self.isDead`))
      (set `self.isFiringBullet` true)
      (`self.FireBullet`)
      (`ActorComponent.Activate` _muzzle true)
      (`AudioComponent.Play` _audiomachinegun 0.0)))
  (:`Released`
    (set `self.isFiringBullet` false)
    (`ActorComponent.Deactivate` _muzzle)
    (`AudioComponent.Stop` _audiomachinegun)))

(fn `DefinePlayerInfo`
  (params (Team :type Name) (Player_ID :type Integer))
  (bind _jet (`self.Jet`))
  (bind _pilotmenu (`self.PilotMenu`))
  (bind (_asbp_hud _bsuccess) (cast `/Game/AircraftWar/blueprint/BP_HUD` (`PlayerController.GetHUD` (`GameplayStatics.GetPlayerController` 0)) :!pure true))
  (bind (_asbp_hud_2 _bsuccess_2) (cast `/Game/AircraftWar/blueprint/BP_HUD` (`PlayerController.GetHUD` (`GameplayStatics.GetPlayerController` 0)) :!pure true))
  (bind _output_get (set `self.Player_ID` Player_ID))
  (`KismetArrayLibrary.Array_Insert` (`self.Tags`) (`KismetStringLibrary.Conv_StringToName` (`KismetStringLibrary.Conv_IntToString` _output_get)))
  (bind _output_get_2 (set `self.Team` Team))
  (switch `name` _output_get_2
    (:`A`
      (`PrimitiveComponent.SetCollisionObjectType` _jet "ECC_Pawn")
      (if _bsuccess
        (set `/Game/AircraftWar/blueprint/BP_HUD.MyTeamA?` true _asbp_hud)
        (set `/Game/AircraftWar/blueprint/BP_HUD.MyPlayer` self _asbp_hud)
        (`PrimitiveComponent.SetCollisionEnabled` _jet "QueryAndPhysics" :!label _label)
        (`SceneComponent.SetVisibility` (`self.DefaultSceneRoot`) true true)
        (set `self.health` (`self.maxHealth`))
        (bind _output_get_3 (set `self.targetSpeed` (`self.MinSpeed`)))
        (set `self.currentSpeed` _output_get_3)
        (set `self.isDead` false)
        (`SceneComponent.SetVisibility` (`self.R_rocket`) true false)
        (`SceneComponent.SetVisibility` (`self.L_rocket`) true false)
        (`/Engine/EditorBlueprintResources/StandardMacros.IsValid` _pilotmenu
          (:`Is Valid`
            (`UserWidget.AddToViewport` _pilotmenu 0)
            (`/Game/AircraftWar/blueprint/UMG_PilotMenu.SetHealth` _pilotmenu (/ (`self.health`) (`self.maxHealth`)))
            (`AudioComponent.Stop` (`self.Alarm`))))))
    (:`B`
      (`PrimitiveComponent.SetCollisionObjectType` _jet "ECC_PhysicsBody")
      (if _bsuccess_2
        (set `/Game/AircraftWar/blueprint/BP_HUD.MyTeamA?` false _asbp_hud_2)
        (set `/Game/AircraftWar/blueprint/BP_HUD.MyPlayer` self _asbp_hud_2)
        (goto _label)))))

(fn `Explode`
  (bind _returnvalue (`self.K2_GetActorLocation`))
  (bind _pilotmenu (`self.PilotMenu`))
  (bind (_asbp_hud _bsuccess) (cast `/Game/AircraftWar/blueprint/BP_HUD` (`PlayerController.GetHUD` (`GameplayStatics.GetPlayerController` 0)) :!pure true))
  (if (not (`self.isDead`))
    (`AudioComponent.Stop` (`self.Alarm`))
    (set `self.isDead` true)
    (set `self.isFiringBullet` false)
    (if _bsuccess
      (set `/Game/AircraftWar/blueprint/BP_HUD.MyPlayer` null _asbp_hud) ; we change value to null to disable hud draw
      (`PrimitiveComponent.SetCollisionEnabled` (`self.Jet`) "NoCollision")
      (`GameplayStatics.SpawnEmitterAtLocation` "/Game/AircraftWar/Effects/P_Explosion.P_Explosion" _returnvalue)
      (`GameplayStatics.SpawnSoundAtLocation` "/Game/AircraftWar/Cues/S_Explosion_Cue.S_Explosion_Cue" _returnvalue (struct) 2.0 1.0 0.0 "/Game/AircraftWar/Cues/A_Attenuation.A_Attenuation" null)
      (`SceneComponent.SetVisibility` (`self.DefaultSceneRoot`) false true)
      (`KismetSystemLibrary.K2_SetTimer` null "RespawnPlayer" (`self.respawnTime`))
      (`GameplayStatics.PlayWorldCameraShake` "/Game/AircraftWar/blueprint/BP_ExplosionShake.BP_ExplosionShake_C" (`self.K2_GetActorLocation`) 6000.0)
      (`/Engine/EditorBlueprintResources/StandardMacros.IsValid` _pilotmenu
        (:`Is Valid`
          (`Widget.RemoveFromParent` _pilotmenu))))))

(fn `FireBullet`
  (bind _returnvalue (`SceneComponent.K2_GetComponentToWorld` (`self.muzzle`)))
  (if (`self.isFiringBullet`)
    (bind _returnvalue_2 (`|SpawnActorFromClass` "/Game/AircraftWar/blueprint/BP_Bullet.BP_Bullet_C" (`KismetMathLibrary.MakeTransform` (.location _returnvalue) (`KismetMathLibrary.MakeRotator` 0.0 (+ (.pitch (.rotation _returnvalue)) (`KismetMathLibrary.RandomFloatInRange` -0.5 1.0)) (+ (.yaw (.rotation _returnvalue)) (`KismetMathLibrary.RandomFloatInRange` -0.5 1.0)))) "Undefined" "OverrideRootScale" null null))
    (`/Engine/EditorBlueprintResources/StandardMacros.IsValid` _returnvalue_2
      (:`Is Valid`
        (`KismetArrayLibrary.Array_Insert` (`Actor.Tags` _returnvalue_2) (`KismetStringLibrary.Conv_StringToName` (`KismetStringLibrary.Conv_IntToString` (`self.Player_ID`))))
        (if (`|EnumEquality` (`PrimitiveComponent.GetCollisionObjectType` (`self.Jet`)) "ECC_Pawn")
          (bind _sphere (`/Game/AircraftWar/blueprint/BP_Bullet.Sphere` _returnvalue_2))
          (`PrimitiveComponent.SetCollisionResponseToChannel` _sphere "ECC_PhysicsBody" "ECR_Overlap")
          (else
            (`PrimitiveComponent.SetCollisionResponseToChannel` _sphere "ECC_Pawn" "ECR_Overlap"))))
      (:`Is Not Valid`
        _))
    (`KismetSystemLibrary.K2_SetTimer` null "FireBullet" (`self.shootingSpeed`))))

(fn `FireRocket`
  (bind _r_rocket (`self.R_rocket`))
  (bind _l_rocket (`self.L_rocket`))
  (bind _pilotmenu (`self.PilotMenu`))
  (bind (_asbp_hud _bsuccess) (cast `/Game/AircraftWar/blueprint/BP_HUD` (`PlayerController.GetHUD` (`GameplayStatics.GetPlayerController` 0)) :!pure true))
  ;[1 1 1] determine which rocket we will shoot , left or right one
  (if (== (`self.RocketSpawnedID`) 0)
    (if (`SceneComponent.IsVisible` _r_rocket)
      (set `self.RocketSpawnedID` 1)
      (set `self.spawnrocketTransform` (`SceneComponent.K2_GetComponentToWorld` _r_rocket))
      (`SceneComponent.SetVisibility` _r_rocket false false)
      (bind _returnvalue (`|SpawnActorFromClass` "/Game/AircraftWar/blueprint/BP_rocket.BP_rocket_C" (`self.spawnrocketTransform`) "Undefined" "OverrideRootScale" null null :!label _label))
      (`/Engine/EditorBlueprintResources/StandardMacros.IsValid` _returnvalue
        (:`Is Valid`
          (set `/Game/AircraftWar/blueprint/BP_rocket.currentSpeed` (`self.currentSpeed`) _returnvalue)
          (`KismetArrayLibrary.Array_Insert` (`Actor.Tags` _returnvalue) (`KismetStringLibrary.Conv_StringToName` (`KismetStringLibrary.Conv_IntToString` (`self.Player_ID`))))
          (if (`|EnumEquality` (`PrimitiveComponent.GetCollisionObjectType` (`self.Jet`)) "ECC_Pawn")
            (bind _sphere (`/Game/AircraftWar/blueprint/BP_rocket.Sphere` _returnvalue))
            (`PrimitiveComponent.SetCollisionResponseToChannel` _sphere "ECC_PhysicsBody" "ECR_Overlap")
            (else
              (`PrimitiveComponent.SetCollisionResponseToChannel` _sphere "ECC_Pawn" "ECR_Overlap")))
          (`GameplayStatics.SpawnSoundAtLocation` "/Game/AircraftWar/Cues/S_Missile_engine_Cue.S_Missile_engine_Cue" (`self.K2_GetActorLocation`) (struct) 3.0 1.0 0.0 "/Game/AircraftWar/Cues/A_Attenuation.A_Attenuation" null)
          ;[1 1 1] we determinate our target from BP_HUD blueprint , our rocket will follow this target actor
          (if _bsuccess
            (set `/Game/AircraftWar/blueprint/BP_rocket.Target` (`/Game/AircraftWar/blueprint/BP_HUD.Target` _asbp_hud) _returnvalue))
          (`KismetSystemLibrary.K2_SetTimer` null "ReloadRocket" (`self.reloadRocketTime`))
          (`GameplayStatics.PlayWorldCameraShake` "/Game/AircraftWar/blueprint/BP_RocketShake.BP_RocketShake_C" (`self.K2_GetActorLocation`) 3000.0)
          (if (and (not (`SceneComponent.IsVisible` (`self.R_rocket`))) (not (`SceneComponent.IsVisible` (`self.L_rocket`))))
            (`/Engine/EditorBlueprintResources/StandardMacros.IsValid` _pilotmenu
              (:`Is Valid`
                (`/Game/AircraftWar/blueprint/UMG_PilotMenu.setRocketState` _pilotmenu false)))))))
    (elif (`SceneComponent.IsVisible` _l_rocket)
      (set `self.RocketSpawnedID` 0)
      (set `self.spawnrocketTransform` (`SceneComponent.K2_GetComponentToWorld` _l_rocket))
      (`SceneComponent.SetVisibility` _l_rocket false false)
      (goto _label))))

(fn `ForwardMovement`
  (params (deltaTime :type "Float (double-precision)"))
  (`self.K2_AddActorLocalOffset` (`KismetMathLibrary.MakeVector` (* deltaTime (`self.currentSpeed`))) true))

(fn `ReloadRocket`
  (bind _pilotmenu (`self.PilotMenu`))
  (if (not (`self.isDead`))
    (`SceneComponent.SetVisibility` (`self.R_rocket`) true false)
    (`SceneComponent.SetVisibility` (`self.L_rocket`) true false)
    (`/Engine/EditorBlueprintResources/StandardMacros.IsValid` _pilotmenu
      (:`Is Valid`
        (`/Game/AircraftWar/blueprint/UMG_PilotMenu.setRocketState` _pilotmenu true)))))

(fn `RespawnPlayer`
  (`self.K2_SetActorTransform` (`self.MySpawnPoint`))
  (`self.DefinePlayerInfo` (`self.Team`) (`self.Player_ID`)))

(fn `RotationControl`
  (params (deltaTime :type "Float (double-precision)"))
  (locals (deltaRot :type "Rotator Structure") (cameraDeltaRot :type "Rotator Structure") (yaw_ratio :type "Float (double-precision)" :default 0.0) (pitch_ratio :type "Float (double-precision)" :default 0.0) (clmp_springArm_drag :type "Float (double-precision)" :default 20.0))
  (bind _clmp_springarm_drag (`local.clmp_springArm_drag`))
  (bind _cameralag (`self.cameraLag`))
  (bind _springarm (`self.SpringArm`))
  (bind _returnvalue (/ (`self.pitch_adder`) (`self.pitch_max`)))
  (bind _returnvalue_2 (/ (`self.yaw_adder`) (`self.yaw_max`)))
  (bind _returnvalue_3 (* _clmp_springarm_drag -1.0))
  (bind (_asbp_hud _bsuccess) (cast `/Game/AircraftWar/blueprint/BP_HUD` (`PlayerController.GetHUD` (`GameplayStatics.GetPlayerController` 0)) :!pure true))
  (bind _output_get (set `local.deltaRot` (`KismetMathLibrary.MakeRotator` (* deltaTime (`self.roll_adder`)) (* deltaTime (`self.pitch_adder`)) (* deltaTime (`self.yaw_adder`)))))
  (`/Engine/EditorBlueprintResources/StandardMacros.IsValid` self
    (:`Is Valid`
      (`self.K2_AddActorLocalRotation` self _output_get true false)
      (bind _output_get_2 (set `local.cameraDeltaRot` (`KismetMathLibrary.MakeRotator` (* _cameralag (`self.roll_adder`) -1.0) (* _cameralag (`self.pitch_adder`) -1.0) (* _cameralag (`self.yaw_adder`) -1.0))))
      (set `SpringArmComponent.TargetArmLength` (* (+ (/ (`self.currentSpeed`) (`self.maxSpeed`)) 0.6) (`self.springarmLengh`)) _springarm)
      (bind (_returnvalue_roll _returnvalue_pitch _returnvalue_yaw) (`KismetMathLibrary.BreakRotator` (`KismetMathLibrary.RInterpTo` (`SceneComponent.RelativeRotation` _springarm) _output_get_2 deltaTime (`self.springArmInterp`))))
      (`SceneComponent.K2_SetRelativeRotation` _springarm (`KismetMathLibrary.MakeRotator` _returnvalue_roll (`KismetMathLibrary.FClamp` _returnvalue_pitch _returnvalue_3 _clmp_springarm_drag) (`KismetMathLibrary.FClamp` _returnvalue_yaw _returnvalue_3 _clmp_springarm_drag)) false false)
      (set `local.yaw_ratio` _returnvalue_2)
      (set `local.pitch_ratio` _returnvalue)
      (bind _output_get_3 (set `self.corssairLocation` (`KismetMathLibrary.MakeVector2D` (* (`KismetMathLibrary.FInterpTo_Constant` (`local.yaw_ratio`) _returnvalue_2 (`GameplayStatics.GetWorldDeltaSeconds`) 10.0) -1.0) (`KismetMathLibrary.FInterpTo_Constant` (`local.pitch_ratio`) _returnvalue (`GameplayStatics.GetWorldDeltaSeconds`) 10.0))))
      (if _bsuccess
        (set `/Game/AircraftWar/blueprint/BP_HUD.CrossairPositionRatio` _output_get_3 _asbp_hud)))))

(fn `SetAlarm`
  (params (TurnOn :type Boolean))
  (bind _alarm (`self.Alarm`))
  (if TurnOn
    (if (not (`AudioComponent.IsPlaying` _alarm))
      (`AudioComponent.Play` _alarm 0.0))
    (elif (`AudioComponent.IsPlaying` _alarm)
      (`AudioComponent.Stop` _alarm))))

(fn `UserConstructionScript`)